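; HUD Blueprint that draws an interaction prompt near the bottom center of the screen.
; The ShowInteract event opens or closes a gate that DrawHUD enters each frame, so the ShowInteractHUD text draws only while enabled.
; Horizontal centering is estimated from the string length.
; Code to create the W_InvMain and Map widgets is present but unconnected, so it never runs.
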(event Collision|EventActorBeginOverlap
  (params (OtherActor :type Actor%20Object%20Reference)))

(event EventTick
  (params (DeltaSeconds :type Float%20%28single-precision%29)))

(event EventDrawHUD
  (params (SizeX :type Integer) (SizeY :type Integer))
  (bind _showinteracthud (Variables|Default|GetshowInteractHUD))
  (Utilities|FlowControl|Gate true
    (:Exit
      (HUD|DrawText _showinteracthud "(R=0.000000,G=0.895000,B=0.628309,A=1.000000)" (- (Math|Conversions|ToFloat(Integer) (/ SizeX 2)) (Math|Conversions|ToFloat(Integer) (* (Utilities|String|Len _showinteracthud) 4))) (+ (Math|Conversions|ToFloat(Integer) SizeY) -1.2e+02) 0 1.0 false))))

(event EventShowInteract
  (params (showInteract? :type Boolean))
  (bind _showinteracthud (Variables|Default|GetshowInteractHUD))
  (if showInteract?
    (Utilities|FlowControl|Gate true) ; enters at Open
    (else
      (Utilities|FlowControl|Gate true) ; enters at Close
    )))

(fn ConstructionScript)